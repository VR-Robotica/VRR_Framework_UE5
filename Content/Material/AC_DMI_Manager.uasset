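; Actor component that manages dynamic material instances (DMIs) for every mesh component on its owner.
; Registering creates one DMI per unique source material, shares it across slots and caches DMI-to-original pairs in a map.
; Setters drive scalar, vector and texture parameters on all DMIs, by index, or by parent material name.
; Unregister and EndPlay restore the original materials and clear the cache.
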(event `Event Init`
  (`self.onInit`))

(event `Event Register`
  (`self.onRegister`))

(event `Event Unregister`
  (`self.onUnregister` :!label _label))

(event `self.ReceiveEndPlay`
  (params (EndPlayReason :type "EEndPlayReason Enum" :default "Destroyed"))
  (goto _label))

(event `Set Custom Scalar`
  (params (Parameter :type Name) (float :type "Float (double-precision)"))
  (`self.onSet Custom Scalar Parameter` Parameter float))

(event `Set Custom Scalar by Index`
  (params (`Material Index` :type Integer) (Parameter :type Name) (float :type "Float (double-precision)"))
  (bind _dmis (`self.get DMIs`))
  (bind _keys (`BlueprintMapLibrary.Map_Keys` _dmis))
  (`MaterialInstanceDynamic.SetScalarParameterValue` (`|GetArrayItem` _keys `Material Index`) Parameter float))

(event `Set Custom Scalar by Parent Name`
  (params (`Parent Name` :type String) (Parameter :type Name) (float :type "Float (double-precision)"))
  (`self.onSet Custom Scalar Parameter by Parent` `Parent Name` Parameter float))

(event `Set Custom Vector4`
  (params (Parameter :type Name) (Vector4 :type "LinearColor Structure"))
  (`self.onSet Custom Vector Parameter` Parameter Vector4))

(event `Set Custom Vector4 by Index`
  (params (`Material Index` :type Integer) (Parameter :type Name) (Vector4 :type "LinearColor Structure"))
  (bind _dmis (`self.get DMIs`))
  (bind _keys (`BlueprintMapLibrary.Map_Keys` _dmis))
  (`MaterialInstanceDynamic.SetVectorParameterValue` (`|GetArrayItem` _keys `Material Index`) Parameter Vector4))

(event `Set Custom Vector4 by Parent Name`
  (params (`Parent Name` :type String) (Parameter :type Name) (Vector4 :type "LinearColor Structure"))
  (`self.onSet Custom Vector4 Parameter by Parent` `Parent Name` Parameter Vector4))

(event `Set Custom Texture2D Parameter`
  (params (Parameter :type Name) (Texture :type "Texture Object Reference"))
  (`self.onSet Custom Texture2D Parameter` Parameter Texture))

(event `Set Custom Texture2D Parameter by Index`
  (params (Parameter :type Name) (`Material Index` :type Integer) (Texture :type "Texture Object Reference"))
  (bind (__materiallibrary_mesh __materiallibrary_dmis) (break `/VRR_Framework/Material/STRUCT_MaterialLibrary` (`self._materialLibrary`)))
  (bind _keys (`BlueprintMapLibrary.Map_Keys` __materiallibrary_dmis))
  (`MaterialInstanceDynamic.SetTextureParameterValue` (`|GetArrayItem` _keys `Material Index`) Parameter Texture))

(event `Set Custom Texture2D Parameter by Parent Name`
  (params (`Parent Name` :type String) (Parameter :type Name) (Texture :type "Texture Object Reference"))
  (bind _target_dmi (`self.get DMIs by Parent Name` `Parent Name`))
  (`MaterialInstanceDynamic.SetTextureParameterValue` _target_dmi Parameter Texture))

(fn `Clear DMIs`
  (bind (__materiallibrary_mesh __materiallibrary_dmis) (break `/VRR_Framework/Material/STRUCT_MaterialLibrary` (`self._materialLibrary`)))
  (`BlueprintMapLibrary.Map_Clear` __materiallibrary_dmis))

(fn `Create DMIs`
  (params (Meshes :type "Array of MeshComponent Object Reference"))
  (locals (_currentMesh :type "MeshComponent Object Reference") (_namingIndex :type Integer) (_index :type String) (_percent :type String) (_originalMaterials_LOCAL :type "Array of MaterialInterface Object Reference") (_currentMaterialIndex :type Integer) (_currentMaterialInstance :type "MaterialInterface Object Reference"))
  (bind (__materiallibrary_mesh __materiallibrary_dmis) (break `/VRR_Framework/Material/STRUCT_MaterialLibrary` (`self._materialLibrary`)))
  (bind (__materiallibrary_mesh_2 __materiallibrary_dmis_2) (break `/VRR_Framework/Material/STRUCT_MaterialLibrary` (`self._materialLibrary`)))
  (bind (__materiallibrary_mesh_3 __materiallibrary_dmis_3) (break `/VRR_Framework/Material/STRUCT_MaterialLibrary` (`self._materialLibrary`)))
  (bind (__materiallibrary_mesh_4 __materiallibrary_dmis_4) (break `/VRR_Framework/Material/STRUCT_MaterialLibrary` (`self._materialLibrary`)))
  (set `local._namingIndex` 0)
  (for _array_element Meshes
    (`/Engine/EditorBlueprintResources/StandardMacros.IsValid` _array_element
      (:`Is Valid`
        (bind _output_get (set `local._currentMesh` _array_element))
        (for (_array_element_2 _array_index) (`MeshComponent.GetMaterials` _output_get)
          (set `local._currentMaterialIndex` _array_index)
          (`/Engine/EditorBlueprintResources/StandardMacros.IsValid` _array_element_2
            (:`Is Valid`
              (set `local._currentMaterialInstance` _array_element_2)
              ;[1 0.5247 0] Check for duplicate DMI origins
              ; (ie material instances - Values)
              (bind _values (`BlueprintMapLibrary.Map_Values` __materiallibrary_dmis_4))
              (if (`KismetArrayLibrary.Array_Contains` _values (`local._currentMaterialInstance`))
                ;[1 1 1] Find previously created DMI (Key) by comparing original material (Value)
                ;
                ; Loop through the Keys and compare the Values with the current material instance
                ; If found, then pass previously made DMI (Key) to the mesh at the current index level
                (bind _keys (`BlueprintMapLibrary.Map_Keys` __materiallibrary_dmis_3))
                (for (_array_element_3 _array_index_2) _keys
                  (bind _values_2 (`BlueprintMapLibrary.Map_Values` __materiallibrary_dmis))
                  (if (== (`local._currentMaterialInstance`) (`|GetArrayItem` _values_2 _array_index_2))
                    (`PrimitiveComponent.SetMaterial` (`local._currentMesh`) (`local._currentMaterialIndex`) _array_element_3)))
                (else
                  ;[1 1 1] Create DMI of our material
                  (bind _returnvalue (`KismetMaterialLibrary.CreateDynamicMaterialInstance` (`local._currentMaterialInstance`) (`KismetStringLibrary.Conv_StringToName` (`KismetStringLibrary.Concat_StrStr` "DMI_" (`KismetStringLibrary.Conv_IntToString` (`local._namingIndex`))))))
                  ;[1 1 1] Apply to appropriate Mesh slot
                  (`PrimitiveComponent.SetMaterial` (`local._currentMesh`) (`local._currentMaterialIndex`) _returnvalue)
                  ;[0 1 0] cache our DMIs with original ref
                  ;
                  ; Key = new DMI
                  ; Value = 'current' orginal material
                  (`BlueprintMapLibrary.Map_Add` __materiallibrary_dmis_2 _returnvalue (`local._currentMaterialInstance`))
                  (set `local._namingIndex` (+ 1 (`local._namingIndex`)))
                  (if (`self.Show Debug`)
                    (`KismetSystemLibrary.PrintString` (`KismetStringLibrary.Concat_StrStr` (`.RightS` (`KismetStringLibrary.Split` (`KismetSystemLibrary.GetDisplayName` (`local._currentMesh`)) " ")) "'s Material Slot [" (`KismetStringLibrary.Conv_IntToString` (`local._currentMaterialIndex`)) "] is " (`KismetSystemLibrary.GetObjectName` (`local._currentMaterialInstance`))) true true (struct :`R` 1.0 :`G` 0.5 :`A` 1.0) 5.0)))))
            (:`Is Not Valid`
              ;[1 0 0] Error out - no material set to mesh's slot
              (if (`self.Show Debug`)
                (`KismetSystemLibrary.PrintString` (`KismetStringLibrary.Concat_StrStr` (`.RightS` (`KismetStringLibrary.Split` (`KismetSystemLibrary.GetDisplayName` (`local._currentMesh`)) " ")) "'s Material Slot [" (`KismetStringLibrary.Conv_IntToString` (`local._currentMaterialIndex`)) "] is NULL") true true (struct :`R` 1.0 :`G` 0.5 :`A` 1.0) 5.0)))))))))

(fn `get Custom Scalar Parameter`
  (params (`custom parameter` :type Name))
  (returns (float :type "Float (double-precision)"))
  (bind _dmis (`self.get DMIs`))
  (bind _keys (`BlueprintMapLibrary.Map_Keys` _dmis))
  (for _array_element _keys
    (bind _returnvalue (`MaterialInstanceDynamic.K2_GetScalarParameterValue` _array_element (`local.custom parameter`)))
    (return _returnvalue)))

(fn `get Custom Vector4 Parameter`
  (params (`custom parameter` :type Name))
  (returns (Vectro4 :type "LinearColor Structure"))
  (bind _dmis (`self.get DMIs`))
  (bind _keys (`BlueprintMapLibrary.Map_Keys` _dmis))
  (for _array_element _keys
    (bind _returnvalue (`MaterialInstanceDynamic.K2_GetVectorParameterValue` _array_element (`local.custom parameter`)))
    (return _returnvalue)))

(fn `get DMIs`
  (returns (DMIs :type "Map of MaterialInstanceDynamic Object Reference to MaterialInterface Object Reference"))
  (bind (__materiallibrary_mesh __materiallibrary_dmis) (break `/VRR_Framework/Material/STRUCT_MaterialLibrary` (`self._materialLibrary`)))
  (bind (__materiallibrary_mesh_2 __materiallibrary_dmis_2) (break `/VRR_Framework/Material/STRUCT_MaterialLibrary` (`self._materialLibrary`)))
  (if (not (> (`BlueprintMapLibrary.Map_Length` __materiallibrary_dmis_2) 0))
    (`self.onInit`))
  (return __materiallibrary_dmis))

(fn `get DMIs by Parent Name`
  (params (name :type String))
  (returns (`Target DMI` :type "MaterialInstanceDynamic Object Reference"))
  (locals (_keyDMIs :type "Array of MaterialInstanceDynamic Object Reference") (_indices :type "Array of Integer") (_target :type "MaterialInstanceDynamic Object Reference"))
  (bind (__materiallibrary_mesh __materiallibrary_dmis) (break `/VRR_Framework/Material/STRUCT_MaterialLibrary` (`self._materialLibrary`)))
  (bind (__materiallibrary_mesh_2 __materiallibrary_dmis_2) (break `/VRR_Framework/Material/STRUCT_MaterialLibrary` (`self._materialLibrary`)))
  (if (`self.Has Initialized`)
    (bind _values (`BlueprintMapLibrary.Map_Values` __materiallibrary_dmis))
    (for (_array_element _array_index) _values
      (if (`KismetStringLibrary.EqualEqual_StrStr` (`KismetSystemLibrary.GetObjectName` _array_element) (`local.name`))
        (bind _keys (`BlueprintMapLibrary.Map_Keys` __materiallibrary_dmis_2))
        (bind _output (`|GetArrayItem` _keys _array_index))
        (`/Engine/EditorBlueprintResources/StandardMacros.IsValid` _output
          (:`Is Valid`
            (bind _output_get (set `local._target` _output))
            (if (`self.Show Debug`)
              (bind _returnvalue (`KismetStringLibrary.Conv_IntToString` _array_index))
              (`KismetSystemLibrary.PrintString` (`KismetStringLibrary.Concat_StrStr` "Found at index[" _returnvalue "] -> " (`KismetSystemLibrary.GetDisplayName` _output_get)))))
          (:`Is Not Valid`
            (if (`self.Show Debug`)
              (`KismetSystemLibrary.PrintString` (`KismetStringLibrary.Concat_StrStr` "DMI Key at index [" _returnvalue "] is NULL!") true true (struct :`R` 1.0 :`A` 1.0)))))))
    (return (`local._target`))
    (else
      (`KismetSystemLibrary.PrintString` "DMI Manager NOT READY"))))

(fn `onInit`
  (bind (__materiallibrary_mesh __materiallibrary_dmis) (break `/VRR_Framework/Material/STRUCT_MaterialLibrary` (`self._materialLibrary`)))
  (bind (__materiallibrary_mesh_2 __materiallibrary_dmis_2) (break `/VRR_Framework/Material/STRUCT_MaterialLibrary` (`self._materialLibrary`)))
  (`|ExecutionSequence`
    (:`then_0`
      (if (`self.Show Debug`)
        (`KismetSystemLibrary.PrintString` ">>>>> Init() <<<<<")))
    (:`then_1`
      (set `self.Has Initialized` false)
      (`|ExecutionSequence`
        (:`then_0`
          ;[1 0.6134 0] Reset Mesh Materials if DMIs previously existed
          (if (> (`BlueprintMapLibrary.Map_Length` __materiallibrary_dmis_2) 0)
            (`self.Event Unregister`)))
        (:`then_1`
          (`self.Event Register`))
        (:`then_2`
          (if (and (> (`BlueprintMapLibrary.Map_Length` __materiallibrary_dmis) 0) (> (`KismetArrayLibrary.Array_Length` (`self._meshComponents`)) 0))
            (set `self.Has Initialized` true))
          (return))))))

(fn `onRegister`
  (`|ExecutionSequence`
    (:`then_0`
      (if (`self.Show Debug`)
        (`KismetSystemLibrary.PrintString` "> onRegister Materials")))
    (:`then_1`
      (bind _output_get (set `self._meshComponents` (`Actor.K2_GetComponentsByClass` (`self.GetOwner`) "/Script/Engine.MeshComponent")))
      (`|ExecutionSequence`
        (:`then_0`
          (if (`self.Show Debug`)
            (`KismetSystemLibrary.PrintString` (`KismetStringLibrary.Concat_StrStr` "> found [" (`KismetStringLibrary.Conv_IntToString` (`KismetArrayLibrary.Array_Length` _output_get)) "] Mesh Components"))
            (for _array_element (`self._meshComponents`)
              (`KismetSystemLibrary.PrintString` (`KismetStringLibrary.Concat_StrStr` "- " (`.RightS` (`KismetStringLibrary.Split` (`KismetSystemLibrary.GetDisplayName` _array_element) " ")))))))
        (:`then_1`
          (`self.Create DMIs` (`self._meshComponents`)))))))

(fn `onSet Custom Scalar Parameter`
  (params (`custom parameter` :type Name) (float :type "Float (double-precision)"))
  (`|ExecutionSequence`
    (:`then_0`
      (if (`self.Show Debug`)
        (`KismetSystemLibrary.PrintString` "onSetCustom Scalar")))
    (:`then_1`
      (bind _dmis (`self.get DMIs`))
      (bind _keys (`BlueprintMapLibrary.Map_Keys` _dmis))
      (for _array_element _keys
        (`MaterialInstanceDynamic.SetScalarParameterValue` _array_element (`local.custom parameter`) (`local.float`))))))

(fn `onSet Custom Scalar Parameter by Parent`
  (params (`Parent Name` :type String) (Parameter :type Name) (Scalar :type "Float (double-precision)"))
  (if (`self.Show Debug`)
    (`KismetSystemLibrary.PrintString` (`KismetStringLibrary.Concat_StrStr` "onSetCustom Scalar by Parent: " `Parent Name`)))
  (bind _target_dmi (`self.get DMIs by Parent Name` `Parent Name`))
  (`/Engine/EditorBlueprintResources/StandardMacros.IsValid` _target_dmi
    (:`Is Valid`
      (if (`self.Show Debug`)
        (`KismetSystemLibrary.PrintString` (`KismetStringLibrary.Concat_StrStr` "> Setting Scalar on " (`KismetSystemLibrary.GetObjectName` _target_dmi))))
      (`MaterialInstanceDynamic.SetScalarParameterValue` _target_dmi Parameter Scalar))))

(fn `onSet Custom Texture2D Parameter`
  (params (Parameter :type Name) (Texture :type "Texture Object Reference"))
  (`|ExecutionSequence`
    (:`then_0`
      (if (`self.Show Debug`)
        (`KismetSystemLibrary.PrintString` "onSetCustom Texture2D")))
    (:`then_1`
      (bind _dmis (`self.get DMIs`))
      (bind _keys (`BlueprintMapLibrary.Map_Keys` _dmis))
      (for _array_element _keys
        (`MaterialInstanceDynamic.SetTextureParameterValue` _array_element (`local.Parameter`) (`local.Texture`))))))

(fn `onSet Custom Vector Parameter`
  (params (`custom parameter` :type Name) (vector4 :type "LinearColor Structure"))
  (`|ExecutionSequence`
    (:`then_0`
      (if (`self.Show Debug`)
        (`KismetSystemLibrary.PrintString` "onSetCustom Vector4")))
    (:`then_1`
      (bind _dmis (`self.get DMIs`))
      (bind _keys (`BlueprintMapLibrary.Map_Keys` _dmis))
      (for _array_element _keys
        (`MaterialInstanceDynamic.SetVectorParameterValue` _array_element (`local.custom parameter`) (`local.vector4`))))))

(fn `onSet Custom Vector4 Parameter by Parent`
  (params (`Parent Name` :type String) (Parameter :type Name) (Vector4 :type "LinearColor Structure"))
  (`|ExecutionSequence`
    (:`then_0`
      (if (`self.Show Debug`)
        (`KismetSystemLibrary.PrintString` (`KismetStringLibrary.Concat_StrStr` "onSetCustom Vector4 by Parent: " `Parent Name`))))
    (:`then_1`
      (bind _target_dmi (`self.get DMIs by Parent Name` `Parent Name`))
      (`/Engine/EditorBlueprintResources/StandardMacros.IsValid` _target_dmi
        (:`Is Valid`
          (if (`self.Show Debug`)
            (`KismetSystemLibrary.PrintString` (`KismetStringLibrary.Concat_StrStr` "> Setting Vector on " (`KismetSystemLibrary.GetObjectName` _target_dmi))))
          (`MaterialInstanceDynamic.SetVectorParameterValue` _target_dmi Parameter Vector4))))))

(fn `onUnregister`
  (`|ExecutionSequence`
    (:`then_0`
      (if (`self.Show Debug`)
        (`KismetSystemLibrary.PrintString` "> onUnregister Materials")))
    (:`then_1`
      (`self.Return Original Materials`))))

(fn `Return Original Materials`
  (locals (_currentMeshComponent :type "MeshComponent Object Reference") (_meshMaterialSet :type "Array of MaterialInterface Object Reference"))
  (bind (__materiallibrary_mesh __materiallibrary_dmis) (break `/VRR_Framework/Material/STRUCT_MaterialLibrary` (`self._materialLibrary`)))
  (bind (__materiallibrary_mesh_2 __materiallibrary_dmis_2) (break `/VRR_Framework/Material/STRUCT_MaterialLibrary` (`self._materialLibrary`)))
  (for _array_element (`self._meshComponents`)
    ;[1 1 1] Get all the DMI materials on the mesh
    (`/Engine/EditorBlueprintResources/StandardMacros.IsValid` _array_element
      (:`Is Valid`
        (bind _output_get (set `local._currentMeshComponent` _array_element))
        ;[1 1 1] Loop through DMIs on the Mesh
        (for (_array_element_2 _array_index) (`MeshComponent.GetMaterials` _output_get)
          (bind _asmaterial_instance_dynamic (cast `MaterialInstanceDynamic` _array_element_2))
          ;[1 0.562 0] Compare mesh's DMI(s) to the DMI-Keys of the cached dictionary map to match the Original Material Instance - Values
          (bind _keys (`BlueprintMapLibrary.Map_Keys` __materiallibrary_dmis_2))
          (for (_array_element_3 _array_index_2) _keys
            (if (`KismetStringLibrary.EqualEqual_StrStr` (`KismetSystemLibrary.GetDisplayName` _array_element_3) (`KismetSystemLibrary.GetDisplayName` _asmaterial_instance_dynamic))
              (bind _values (`BlueprintMapLibrary.Map_Values` __materiallibrary_dmis))
              ;[0 1 0] Apply the original material
              (`|ExecutionSequence`
                (:`then_0`
                  (if (`self.Show Debug`)
                    (bind _output (`|GetArrayItem` _values _array_index_2))
                    (`KismetSystemLibrary.PrintString` (`KismetSystemLibrary.GetObjectName` _output))))
                (:`then_1`
                  (`PrimitiveComponent.SetMaterial` (`local._currentMeshComponent`) _array_index _output)))))))))
  (`self.Clear DMIs`))

(fn `Validate Master Material`
  (params (`Material Name` :type String))
  (returns (isValid :type Boolean) (index :type Integer))
  (locals (_isValid :type Boolean :default false) (_index :type Integer :default -1))
  (bind (__materiallibrary_mesh __materiallibrary_dmis) (break `/VRR_Framework/Material/STRUCT_MaterialLibrary` (`self._materialLibrary`)))
  (bind _values (`BlueprintMapLibrary.Map_Values` __materiallibrary_dmis))
  (for (_array_element _array_index) _values
    (if (`KismetStringLibrary.EqualEqual_StrStr` (`KismetSystemLibrary.GetObjectName` _array_element) (`local.Material Name`))
      (set `local._isValid` true)
      (set `local._index` _array_index)
      (break)))
  (return (`local._isValid`) (`local._index`)))